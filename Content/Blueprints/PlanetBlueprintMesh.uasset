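; Procedural planet actor that builds its terrain mesh with Geometry Script in the construction script.
; Resets the DynamicMeshComponent, appends a sphere box sized by Radius and PlanetScale, then tessellates it.
; Layers large and small Perlin noise, tessellates again, then adds detail noise.
; Noise magnitude and frequency derive from unscaled Radius and per-layer variables, so PlanetScale affects only the base sphere size.
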(event EventBeginPlay)

(event Collision|EventActorBeginOverlap
  (params (OtherActor :type Actor%20Object%20Reference)))

(event EventTick
  (params (DeltaSeconds :type Float%20%28single-precision%29)))

(fn ConstructionScript
  (bind _returnvalue (DynamicMeshComponent|GetDynamicMesh (Variables|DynamicMeshActor|GetDynamicMeshComponent)))
  (bind _output_get (Variables|Default|SetDynamicMesh _returnvalue))
  (DynamicMesh|Reset _output_get)
  (bind _returnvalue_2 (Class|GeometryScriptLibraryMeshPrimitiveFunctions|AppendSphereBox :TargetMesh (Variables|Default|GetDynamicMesh) :PrimitiveOptions (Utilities|Struct|MakeGeometryScriptPrimitiveOptions "PerFace") :Radius (* (Variables|Default|GetRadius) (Variables|Default|GetPlanetScale)) :StepsX 8 :StepsY 8 :StepsZ 8 :Debug 0))
  (bind _returnvalue_3 (Class|GeometryScriptLibraryMeshSubdivideFunctions|ApplyUniformTessellation _returnvalue_2 4 0))
  ;[0.15 0.15 0.15 0.5] Large Noise
  (bind _returnvalue_4 (Class|GeometryScriptLibraryMeshDeformFunctions|ApplyPerlinNoisetoMesh :TargetMesh _returnvalue_3 :Options (Utilities|Struct|MakeGeometryScriptPerlinNoiseOptions (Utilities|Struct|MakeGeometryScriptPerlinNoiseLayerOptions (/ (Variables|Default|GetRadius) (Math|Float|MakeLiteralFloat (Variables|Default|GetLargeNoiseMagnitude))) (/ (Math|Float|MakeLiteralFloat (Variables|Default|GetLargeNoiseFreqMagnitude)) (Variables|Default|GetRadius)) "0.000000,0.000000,0.000000" 0) true "FullMeshSelection") :Debug 0))
  ;[0.15 0.15 0.15 0.5] Small Noise
  (bind _returnvalue_5 (Class|GeometryScriptLibraryMeshDeformFunctions|ApplyPerlinNoisetoMesh :TargetMesh _returnvalue_4 :Options (Utilities|Struct|MakeGeometryScriptPerlinNoiseOptions (Utilities|Struct|MakeGeometryScriptPerlinNoiseLayerOptions (/ (Variables|Default|GetRadius) (Math|Float|MakeLiteralFloat (Variables|Default|GetSmallNoiseMagnitude))) (/ (Math|Float|MakeLiteralFloat (Variables|Default|GetSmallNoiseFreqMagnitude)) (Variables|Default|GetRadius)) "0.000000,0.000000,0.000000" 0) true "FullMeshSelection") :Debug 0))
  ;[0.15 0.15 0.15 0.5] Tesselation
  (bind _returnvalue_6 (Class|GeometryScriptLibraryMeshSubdivideFunctions|ApplyUniformTessellation _returnvalue_5 2 0))
  ;[0.15 0.15 0.15 0.5] Detail Noise
  (Class|GeometryScriptLibraryMeshDeformFunctions|ApplyPerlinNoisetoMesh :TargetMesh _returnvalue_6 :Options (Utilities|Struct|MakeGeometryScriptPerlinNoiseOptions (Utilities|Struct|MakeGeometryScriptPerlinNoiseLayerOptions (/ (Variables|Default|GetRadius) (Math|Float|MakeLiteralFloat (Variables|Default|GetDetailNoiseMagnitude))) (/ (Math|Float|MakeLiteralFloat (Variables|Default|GetDetailNoiseFreqMagnitude)) (Variables|Default|GetRadius)) "0.000000,0.000000,0.000000" 0) true "FullMeshSelection") :Debug 0))